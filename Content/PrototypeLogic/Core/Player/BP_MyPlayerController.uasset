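; Player controller that handles the Interact input and the pause menu, working through BP_MainGameMode, which it caches in the construction script.
; Interact, unless blocked by StopInteract, triggers the current trigger object or otherwise releases a held single object.
; The Z key opens a pause window via the UI manager, and pausing and continuing toggle input mode, cursor and game pause.
; Log helpers forward messages to the game mode's debug manager.
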(event `self.ReceiveBeginPlay`)

(event `Key|Z`
  (params (Key :type "Key Structure"))
  (:`Pressed`
    (`self.ShowPauseMenuWindow`)))

(event `InputAction|Interact`
  (params (Key :type "Key Structure"))
  (:`Pressed`
    (if (not (`self.bStopInteract`))
      (if (`/Game/PrototypeLogic/Core/Player/BP_MainGameMode.bCanInteract` (`self.MainGameMode`))
        (`/Game/PrototypeLogic/Core/Managers/TriggerLogic/BP_TriggerBase.Interact` (`/Game/PrototypeLogic/Core/Player/BP_MainGameMode.TriggerObject` (`self.MainGameMode`)))
        (elif (not (`/Game/PrototypeLogic/Core/Player/BP_MyCharacter.bCanGrabSingleObjects` (`/Game/PrototypeLogic/Core/Player/BP_MainGameMode.GamePlayerCharacter` (`self.MainGameMode`))))
          (`/Game/PrototypeLogic/Core/Player/BP_MyCharacter.ReleaseSingleObject` (`/Game/PrototypeLogic/Core/Player/BP_MainGameMode.GamePlayerCharacter` (`self.MainGameMode`)))
          (else
            (`self.DebugLog` "Nothing to drop")))))))

(fn `ContinueGame`
  (`/Game/PrototypeLogic/Core/Managers/UIManagerLogic/UIManagerComponent.CloseWindow` (`/Game/PrototypeLogic/Core/Player/BP_MainGameMode.UIManagerComponent` (`self.MainGameMode`)))
  (`self.UnpauseGame`))

(fn `DebugLog`
  (params (Message :type String))
  (`/Game/PrototypeLogic/Core/Managers/DebugManagerLogic/DebugManagerComponent.DebugLog` (`/Game/PrototypeLogic/Core/Player/BP_MainGameMode.DebugManagerComponent` (`self.MainGameMode`)) self Message))

(fn `ErrorLog`
  (params (Message :type String))
  (`/Game/PrototypeLogic/Core/Managers/DebugManagerLogic/DebugManagerComponent.ErrorLog` (`/Game/PrototypeLogic/Core/Player/BP_MainGameMode.DebugManagerComponent` (`self.MainGameMode`)) self Message))

(fn `PauseGame`
  (`WidgetBlueprintLibrary.SetInputMode_UIOnlyEx` self null)
  (set `self.bShowMouseCursor` true)
  (`GameplayStatics.SetGamePaused` true))

(fn `ShowPauseMenuWindow`
  (`/Game/PrototypeLogic/Core/Managers/UIManagerLogic/UIManagerComponent.ShowWindowNew` (`/Game/PrototypeLogic/Core/Player/BP_MainGameMode.UIManagerComponent` (`self.MainGameMode`)) "NewEnumerator5")
  (`self.PauseGame`))

(fn `SuccessLog`
  (params (Message :type String))
  (`/Game/PrototypeLogic/Core/Managers/DebugManagerLogic/DebugManagerComponent.SuccessLog` (`/Game/PrototypeLogic/Core/Player/BP_MainGameMode.DebugManagerComponent` (`self.MainGameMode`)) self Message))

(fn `UnpauseGame`
  (`WidgetBlueprintLibrary.SetInputMode_GameOnly` self)
  (`GameplayStatics.SetGamePaused` false)
  (set `self.bShowMouseCursor` false))

(fn `UserConstructionScript`
  (bind _asbp_main_game_mode (cast `/Game/PrototypeLogic/Core/Player/BP_MainGameMode` (`GameplayStatics.GetGameMode`)))
  (set `self.MainGameMode` _asbp_main_game_mode))

(fn `WarningLog`
  (params (Message :type String))
  (`/Game/PrototypeLogic/Core/Managers/DebugManagerLogic/DebugManagerComponent.WarningLog` (`/Game/PrototypeLogic/Core/Player/BP_MainGameMode.DebugManagerComponent` (`self.MainGameMode`)) self Message))