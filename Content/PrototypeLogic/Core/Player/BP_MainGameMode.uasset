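; Main game mode that serves both the main menu and gameplay levels, telling them apart by level name.
; Construction picks the default pawn, then BeginPlay either shows the menu or sets up the HUD, input mode and player references.
; In gameplay it binds manager component events: dialogue toggles movement, interaction and cursor, popups update the information HUD, and tasks toggle pause-menu buttons.
; AI controllers get the first AICharacters entry as default pawn.
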(event `self.ReceiveBeginPlay`
  ;[1 1 1] Main Game Architecture
  (`|ExecutionSequence`
    (:`then_0`
      (`self.SetPlayerController`))
    (:`then_1`
      (if (`self.bIsGame`)
        (`self.OnGameEvent_BeginPlay`)
        (else
          (`self.OnMainMenuEvent_BeginPlay`))))))

(event `OnDialogueStarted_Event`
  ;[1 1 1] Binds
  ;;[1 1 1] Bind Dialog Manager Component
  (`/Game/PrototypeLogic/Core/Player/BP_MyCharacter.DisableFullMovement` (`self.GamePlayerCharacter`))
  (set `/Game/PrototypeLogic/Core/Player/BP_MyPlayerController.bStopInteract` true (`self.MainPlayerController`))
  (`WidgetBlueprintLibrary.SetInputMode_GameAndUIEx` (`self.MainPlayerController`) null)
  (set `PlayerController.bShowMouseCursor` true (`self.MainPlayerController`)))

(event `BindDialogueManagerComponent_Event`
  (bind _dialoguemanagercomponent (`self.DialogueManagerComponent`))
  ;[1 1 1] Binds
  ;;[1 1 1] Bind Dialog Manager Component
  (`|ExecutionSequence`
    (:`then_0`
      (add `/Game/PrototypeLogic/Core/Managers/DialogueManagerLogic/DialogueManagerComponent.OnDialogueStarted` _dialoguemanagercomponent (delegate `OnDialogueStarted_Event`)))
    (:`then_1`
      (add `/Game/PrototypeLogic/Core/Managers/DialogueManagerLogic/DialogueManagerComponent.OnDialogueFinished` _dialoguemanagercomponent (delegate `OnDialogueFinished_Event`)))))

(event `OnGameEvent_Initialize`
  ;[1 1 1] Main Game Architecture
  (set `self.DefaultPawnClass` "/Game/PrototypeLogic/Core/Player/BP_MyCharacter.BP_MyCharacter_C"))

(event `OnDialogueFinished_Event`
  ;[1 1 1] Binds
  ;;[1 1 1] Bind Dialog Manager Component
  (`/Game/PrototypeLogic/Core/Player/BP_MyCharacter.EnableFullMovement` (`self.GamePlayerCharacter`))
  (`WidgetBlueprintLibrary.SetInputMode_GameOnly` (`self.MainPlayerController`))
  (set `PlayerController.bShowMouseCursor` false (`self.MainPlayerController`))
  (set `/Game/PrototypeLogic/Core/Player/BP_MyPlayerController.bStopInteract` false (`self.MainPlayerController`)))

(event `OnGameEvent_BeginPlay`
  (bind _mainplayercontroller (`self.MainPlayerController`))
  ;[1 1 1] Main Game Architecture
  (`|ExecutionSequence`
    (:`then_0`
      (`self.InitHUDandUI`)
      (`self.InitInteractInformationPopup`))
    (:`then_1`
      (`WidgetBlueprintLibrary.SetInputMode_GameOnly` _mainplayercontroller)
      (set `PlayerController.bShowMouseCursor` false _mainplayercontroller)
      (bind _asbp_my_character (cast `/Game/PrototypeLogic/Core/Player/BP_MyCharacter` (`GameplayStatics.GetPlayerCharacter` 0)))
      (set `self.GamePlayerCharacter` _asbp_my_character))
    (:`then_2`
      (`self.BindDialogueManagerComponent_Event`)
      (`self.BindPopupManagerComponent_Event`)
      (`self.BindTaskManagerComponent`))))

(event `BindPopupManagerComponent_Event`
  (bind _popupmanagercomponent (`self.PopupManagerComponent`))
  ;[1 1 1] Binds
  ;;[1 1 1] Bind Popup Manager Component
  (`|ExecutionSequence`
    (:`then_0`
      (add `/Game/PrototypeLogic/Core/Managers/PopupManagerLogic/PopupManagerComponent.OnPopupShow` _popupmanagercomponent (delegate `OnPopupShowed_Event`)))
    (:`then_1`
      (add `/Game/PrototypeLogic/Core/Managers/PopupManagerLogic/PopupManagerComponent.OnPopupHide` _popupmanagercomponent (delegate `OnPopupHide_Event`)))
    (:`then_2`
      (add `/Game/PrototypeLogic/Core/Managers/PopupManagerLogic/PopupManagerComponent.OnHideAllPopupsImmediately` _popupmanagercomponent (delegate `OnPopupHideImmediately_Event`)))))

(event `OnPopupShowed_Event`
  (params (Popup :type "/Game/PrototypeLogic/Core/WidgetLogic/BaseLogic/Popup_Base Object Reference"))
  ;[1 1 1] Binds
  ;;[1 1 1] Bind Popup Manager Component
  (`/Game/PrototypeLogic/Core/WidgetLogic/HUD/HUD_Information.AddPopupToHUD` (`self.InformationHUD`) Popup))

(event `OnMainMenuEvent_Initialize`
  ;[1 1 1] Main Game Architecture
  (set `self.DefaultPawnClass` "/Game/PrototypeLogic/Core/Player/BP_MainMenuPawn.BP_MainMenuPawn_C"))

(event `OnPopupHide_Event`
  ;[1 1 1] Binds
  ;;[1 1 1] Bind Popup Manager Component
  (`/Game/PrototypeLogic/Core/WidgetLogic/HUD/HUD_Information.RemovePopupFromHUD` (`self.InformationHUD`)))

(event `OnMainMenuEvent_BeginPlay`
  ;[1 1 1] Main Game Architecture
  (`/Game/PrototypeLogic/Core/Managers/UIManagerLogic/UIManagerComponent.InitializeWindows` (`self.UIManagerComponent`))
  (`self.ShowMainMenu`))

(event `OnPopupHideImmediately_Event`
  ;[1 1 1] Binds
  ;;[1 1 1] Bind Popup Manager Component
  (`/Game/PrototypeLogic/Core/WidgetLogic/HUD/HUD_Information.RemovePopupFromHUD` (`self.InformationHUD`)))

(event `BindTaskManagerComponent`
  ;[1 1 1] Binds
  ;;[1 1 1] Bind Task Manager Component
  (add `/Game/PrototypeLogic/Core/Managers/TaskManagerLogic/TaskManagerComponent.OnSetVisibleTaskControlButtons` (`self.TaskManagerComponent`) (delegate `OnSetVisibleTaskControlButtons_Event`)))

(event `OnSetVisibleTaskControlButtons_Event`
  (params (Visibility :type Boolean))
  (bind _buttonsmanagercomponent (`self.ButtonsManagerComponent`))
  (bind _pausemenubuttons (`/Game/PrototypeLogic/Core/Managers/UIButtonsManagerLogic/ButtonsManagerComponent.PauseMenuButtons` _buttonsmanagercomponent))
  ;[1 1 1] Binds
  ;;[1 1 1] Bind Task Manager Component
  (`|ExecutionSequence`
    (:`then_0`
      (`/Game/PrototypeLogic/Core/Managers/UIButtonsManagerLogic/ButtonsManagerComponent.SetButtonVisibility` _buttonsmanagercomponent _pausemenubuttons 1 Visibility))
    (:`then_1`
      (`/Game/PrototypeLogic/Core/Managers/UIButtonsManagerLogic/ButtonsManagerComponent.SetButtonVisibility` _buttonsmanagercomponent _pausemenubuttons 2 Visibility))))

(fn `CallInitEvents`
  (if (`self.bIsGame`)
    (`self.OnGameEvent_Initialize`)
    (else
      (`self.OnMainMenuEvent_Initialize`))))

(fn `GetDefaultPawnClassForController`
  (params (InController :type "Controller Object Reference"))
  (returns (ReturnValue :type "Object Class Reference"))
  (if (`Controller.IsPlayerController` InController)
    (bind _returnvalue (`parent.GetDefaultPawnClassForController` InController))
    (return _returnvalue)
    (else
      (for _array_element (`self.AICharacters`)
        (return _array_element)))))

(fn `InitHUDandUI`
  (bind _uimanagercomponent (`self.UIManagerComponent`))
  (`/Game/PrototypeLogic/Core/Managers/UIManagerLogic/UIManagerComponent.InitializeWindows` _uimanagercomponent)
  (`/Game/PrototypeLogic/Core/Managers/UIManagerLogic/UIManagerComponent.InitializeHUDs` _uimanagercomponent)
  (bind _return (`/Game/PrototypeLogic/Core/Managers/UIManagerLogic/UIManagerComponent.GetHUD` _uimanagercomponent "NewEnumerator1"))
  (bind _ashud_information (cast `/Game/PrototypeLogic/Core/WidgetLogic/HUD/HUD_Information` _return))
  (set `self.InformationHUD` _ashud_information)
  (`/Game/PrototypeLogic/Core/Managers/UIManagerLogic/UIManagerComponent.ShowHUD` _uimanagercomponent "NewEnumerator1"))

(fn `InitInteractInformationPopup`
  (bind _returnvalue (`|CreateWidget` "/Game/PrototypeLogic/Core/WidgetLogic/Popups/Information/InteractInformation_Popup.InteractInformation_Popup_C"))
  (set `self.InteractInformationPopup` _returnvalue))

(fn `SetIsGame`
  (bind _returnvalue (`GameplayStatics.GetCurrentLevelName` true))
  (if (`KismetStringLibrary.EqualEqual_StrStr` _returnvalue "Level-00_MainMenu")
    (set `self.bIsGame` false)
    (else
      (set `self.bIsGame` true))))

(fn `SetPlayerController`
  (bind _asbp_my_player_controller (cast `/Game/PrototypeLogic/Core/Player/BP_MyPlayerController` (`GameplayStatics.GetPlayerController` 0)))
  (set `self.MainPlayerController` _asbp_my_player_controller))

(fn `ShowMainMenu`
  (bind _return (`/Game/PrototypeLogic/Core/Managers/UIManagerLogic/UIManagerComponent.ShowWindowNew` (`self.UIManagerComponent`) "NewEnumerator0"))
  (`WidgetBlueprintLibrary.SetInputMode_UIOnlyEx` (`self.MainPlayerController`) _return)
  (set `PlayerController.bShowMouseCursor` true (`self.MainPlayerController`)))

(fn `UserConstructionScript`
  (`|ExecutionSequence`
    (:`then_0`
      (`self.SetIsGame`))
    (:`then_1`
      (`self.CallInitEvents`))))