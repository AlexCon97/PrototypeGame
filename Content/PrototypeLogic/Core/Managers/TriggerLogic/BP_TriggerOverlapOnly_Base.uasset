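; Base trigger actor that enables player interaction purely through overlap.
; On begin overlap it sets CanInteract on the main game mode, registers itself as TriggerObject and blocks the player character's ray via IsRayBlocked.
; On end overlap it clears both flags but still leaves itself assigned as TriggerObject.
; It calls parent implementations and does not filter the overlapping actor.
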(event `self.ReceiveBeginPlay`
  (`parent.ReceiveBeginPlay`))

(event `self.ReceiveActorBeginOverlap`
  (params (OtherActor :type "Actor Object Reference"))
  (bind _maingamemode (`self.MainGameMode`))
  (`parent.ReceiveActorBeginOverlap` OtherActor)
  (set `/Game/PrototypeLogic/Core/Player/BP_MainGameMode.bCanInteract` true _maingamemode)
  (set `/Game/PrototypeLogic/Core/Player/BP_MainGameMode.TriggerObject` self _maingamemode)
  (set `/Game/PrototypeLogic/Core/Player/BP_MyCharacter.bIsRayBlocked` true (`/Game/PrototypeLogic/Core/Player/BP_MainGameMode.GamePlayerCharacter` (`self.MainGameMode`))))

(event `self.ReceiveActorEndOverlap`
  (params (OtherActor :type "Actor Object Reference"))
  (bind _maingamemode (`self.MainGameMode`))
  (`parent.ReceiveActorEndOverlap` OtherActor)
  (set `/Game/PrototypeLogic/Core/Player/BP_MainGameMode.bCanInteract` false _maingamemode)
  (set `/Game/PrototypeLogic/Core/Player/BP_MainGameMode.TriggerObject` self _maingamemode)
  (set `/Game/PrototypeLogic/Core/Player/BP_MyCharacter.bIsRayBlocked` false (`/Game/PrototypeLogic/Core/Player/BP_MainGameMode.GamePlayerCharacter` (`self.MainGameMode`))))

(fn `UserConstructionScript`
  (`parent.UserConstructionScript`))