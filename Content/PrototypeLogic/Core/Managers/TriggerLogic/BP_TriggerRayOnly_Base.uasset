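; BP_TriggerRayOnly_Base is a base trigger that shows interaction text while an interaction ray overlaps it.
; RayBeginOverlap sets IsRayOverlapped, adds the game mode's InteractInformationPopup to the InformationHUD and fills it with placeholder text meant to be replaced through SetInteractionText.
; RayEndOverlap clears the flag and removes the popup from the HUD.
; BeginPlay and the construction script only call their parents.
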(event `self.ReceiveBeginPlay`
  (`parent.ReceiveBeginPlay`))

(fn `AddInteractionText`
  (bind _maingamemode (`self.MainGameMode`))
  (`/Game/PrototypeLogic/Core/WidgetLogic/HUD/HUD_Information.AddInterationInformation` (`/Game/PrototypeLogic/Core/Player/BP_MainGameMode.InformationHUD` _maingamemode) (`/Game/PrototypeLogic/Core/Player/BP_MainGameMode.InteractInformationPopup` _maingamemode)))

(fn `RayBeginOverlap`
  (set `self.bIsRayOverlapped` true)
  (`self.AddInteractionText`)
  (`self.SetInteractionText` "Use SetInteractionText Method to set this text"))

(fn `RayEndOverlap`
  (set `self.bIsRayOverlapped` false)
  (`self.RemoveInteractionText`))

(fn `RemoveInteractionText`
  (`/Game/PrototypeLogic/Core/WidgetLogic/HUD/HUD_Information.RemoveInterationInformation` (`/Game/PrototypeLogic/Core/Player/BP_MainGameMode.InformationHUD` (`self.MainGameMode`))))

(fn `SetInteractionText`
  (params (InteractionText :type Text))
  (`/Game/PrototypeLogic/Core/WidgetLogic/Popups/Information/InteractInformation_Popup.SetInteractionText` (`/Game/PrototypeLogic/Core/Player/BP_MainGameMode.InteractInformationPopup` (`self.MainGameMode`)) InteractionText))

(fn `UserConstructionScript`
  (`parent.UserConstructionScript`))