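; BP_TriggerBase is a base actor for triggers that can animate itself by moving and rotating.
; On BeginPlay it derives start and end positions from the root's location plus an offset and sets the movement timeline's play rate.
; Optional flags start timelines that lerp the root's world location between those points and its world rotation from zero to a target angle.
; Interact and the overlap events are empty stubs.
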(event `self.ReceiveBeginPlay`
  (`|ExecutionSequence`
    (:`then_0`
      ;[1 1 1] Set Start End Pos of Moving Anim
      (bind _output_get (set `self.StartPos` (`SceneComponent.K2_GetComponentLocation` (`self.SceneRoot`))))
      (set `self.EndPos` (+ _output_get (`self.LengthMovingWay`))))
    (:`then_1`
      (`TimelineComponent.SetPlayRate` (`self.MovingTimeline`) (`self.PlayMovingRate`)))
    (:`then_2`
      (if (`self.bIsMovingAnimCycling`)
        (bind (_direction _movingtrack) (`Timeline|MovingTimeline`)
          (:`Update`
            (`SceneComponent.K2_SetWorldLocation` (`self.SceneRoot`) (`KismetMathLibrary.VLerp` (`self.StartPos`) (`self.EndPos`) _movingtrack) false false)))))
    (:`then_3`
      (if (`self.bIsRotatingAnimCycling`)
        (bind (_direction_2 _rotatingtrack) (`Timeline|RotatingTimeline`)
          (:`Update`
            (`SceneComponent.K2_SetWorldRotation` (`self.SceneRoot`) (`KismetMathLibrary.RLerp` (struct) (`self.RotatingAngle`) _rotatingtrack) false false)))))))

(event `self.ReceiveActorBeginOverlap`
  (params (OtherActor :type "Actor Object Reference")))

(event `self.ReceiveActorEndOverlap`
  (params (OtherActor :type "Actor Object Reference")))

(fn `Interact`)

(fn `UserConstructionScript`)