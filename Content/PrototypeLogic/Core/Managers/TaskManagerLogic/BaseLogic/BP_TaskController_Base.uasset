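; Base task actor that gathers main and addition task components into arrays and name maps at construction.
; Main tasks run sequentially until all complete and the finished popup shows; addition task completions are only counted.
; Overlap toggles a description popup, while interacting makes it the current task and hides spawned tasks.
; Start, cancel, reload and complete drive TaskManager, HUD popups and actors the task spawned; save, restore and preview only log.
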(event `AdditionTaskCompleted_Event`
  ;[1 1 1] Bind OnAdditionTaskCompleted Event. Call when AdditionTask will complete
  (bind _result (`/Engine/EditorBlueprintResources/StandardMacros.IncrementInt` (`self.CompletedAdditionTasksAmount`))
    (:`  `
      (set `self.CompletedAdditionTasksAmount` _result))))

(event `self.ReceiveBeginPlay`
  (`parent.ReceiveBeginPlay`)
  (`|ExecutionSequence`
    (:`then_0`
      ;[1 1 1] Bind OnAdditionTaskCompleted Event. Call when AdditionTask will complete
      (for _array_element (`self.AdditionTasks`)
        (add `/Game/PrototypeLogic/Core/Managers/TaskManagerLogic/BaseLogic/AdditionTask_Base.OnAdditionTaskCompleted` _array_element (delegate `AdditionTaskCompleted_Event`))))
    (:`then_1`
      ;[1 1 1] Bind OnMainTaskCompleted Event. Call when MainTask will complete
      (for _array_element_2 (`self.MainTasks`)
        (add `/Game/PrototypeLogic/Core/Managers/TaskManagerLogic/BaseLogic/MainTask_Base.OnMainTaskCompleted` _array_element_2 (delegate `MainTaskCompleted_Event`))))))

(event `MainTaskCompleted_Event`
  ;[1 1 1] Bind OnMainTaskCompleted Event. Call when MainTask will complete
  (bind _result (`/Engine/EditorBlueprintResources/StandardMacros.IncrementInt` (`self.CompletedMainTasksAmount`))
    (:`  `
      (set `self.CompletedMainTasksAmount` _result)
      (if (`self.IsMainTasksFullyCompleted`)
        (`self.SuccessLog` "AllMainTasksCompleted")
        (`self.CompleteTask`)
        (else
          (`/Game/PrototypeLogic/Core/Managers/TaskManagerLogic/BaseLogic/Task_Base.StartTask` (`|GetArrayItem` (`self.MainTasks`) (`self.CompletedMainTasksAmount`)))
          (`self.DebugLog` "Next Main Task Started. BP_TaskControllerBase, MainTaskCompleted_Event"))))))

(event `self.ReceiveActorBeginOverlap`
  (params (OtherActor :type "Actor Object Reference"))
  (`parent.ReceiveActorBeginOverlap` OtherActor)
  (`self.ShowDescriptionTaskPopup`))

(event `self.ReceiveActorEndOverlap`
  (params (OtherActor :type "Actor Object Reference"))
  (`parent.ReceiveActorEndOverlap` OtherActor)
  (`self.HideDescriptionTaskPopup`))

(fn `CancelAdditionTasks`
  (bind _additiontasks (`self.AdditionTasks`))
  (if (> (`KismetArrayLibrary.Array_Length` _additiontasks) 0)
    (for _array_element _additiontasks
      (`/Game/PrototypeLogic/Core/Managers/TaskManagerLogic/BaseLogic/Task_Base.CancelTask` _array_element))
    (`self.DebugLog` "Parent:Cancel Addition Tasks")))

(fn `CancelMainTasks`
  (for _array_element (`self.MainTasks`)
    (`/Game/PrototypeLogic/Core/Managers/TaskManagerLogic/BaseLogic/Task_Base.CancelTask` _array_element)))

(fn `CancelTask`
  (bind _taskmanager (`self.TaskManager`))
  (`|ExecutionSequence`
    (:`then_0`
      (`self.CancelMainTasks`)
      (`self.CancelAdditionTasks`))
    (:`then_1`
      (`/Game/PrototypeLogic/Core/Managers/TaskManagerLogic/TaskManagerComponent.UnHideSpawnedTasks` _taskmanager))
    (:`then_2`
      (`self.HideDescriptionTaskPopup`))
    (:`then_3`
      (`/Game/PrototypeLogic/Core/Managers/TaskManagerLogic/TaskManagerComponent.SetVisibleTaskControlButtons` _taskmanager false))
    (:`then_4`
      (set `self.bIsTaskActive` false))
    (:`then_5`
      (`self.RemoveInteractionText`))
    (:`then_6`
      (`/Game/PrototypeLogic/Core/Managers/PopupManagerLogic/PopupManagerComponent.HideAllPopupsImmediately` (`/Game/PrototypeLogic/Core/Player/BP_MainGameMode.PopupManagerComponent` (`self.MainGameMode`))))
    (:`then_7`
      (`self.DestroySpawnedActors`))))

(fn `CompleteAdditionTaskModule`
  (params (TaskName :type Name))
  (bind (_value _returnvalue) (`BlueprintMapLibrary.Map_Find` (`self.AdditionTasksGroup`) TaskName))
  (if _returnvalue
    (`/Game/PrototypeLogic/Core/Managers/TaskManagerLogic/BaseLogic/Task_Base.CompleteTask` _value)
    (else
      ;[1 1 1] DebugMessage
      (bind _output_get (set `self.DebugText` "Didn't find "))
      (`self.ErrorLog` (`KismetStringLibrary.Concat_StrStr` (`KismetStringLibrary.Concat_StrStr` _output_get (`KismetStringLibrary.Conv_NameToString` TaskName)) " in AdditionTasksGroup")))))

(fn `CompleteMainTaskModule`
  (params (TaskName :type Name))
  (bind (_value _returnvalue) (`BlueprintMapLibrary.Map_Find` (`self.MainTasksGroup`) TaskName))
  (if _returnvalue
    (`/Game/PrototypeLogic/Core/Managers/TaskManagerLogic/BaseLogic/Task_Base.CompleteTask` _value)
    (`self.ResetMainTaskValues`)
    (else
      ;[1 1 1] DebugMessage
      (bind _output_get (set `self.DebugText` "Didn't find "))
      (`self.ErrorLog` (`KismetStringLibrary.Concat_StrStr` (`KismetStringLibrary.Concat_StrStr` _output_get (`KismetStringLibrary.Conv_NameToString` TaskName)) " in MainTasksGroup")))))

(fn `CompleteTask`
  (bind _taskmanager (`self.TaskManager`))
  (`self.DebugLog` "Parent:TaskCompletedFully")
  (`|ExecutionSequence`
    (:`then_0`
      (`/Game/PrototypeLogic/Core/WidgetLogic/HUD/HUD_Information.RemoveTaskPopupBaseFromHUD` (`/Game/PrototypeLogic/Core/Player/BP_MainGameMode.InformationHUD` (`self.MainGameMode`))))
    (:`then_1`
      (`self.ShowFinishedTaskPopup`)
      (`/Game/PrototypeLogic/Core/Managers/TaskManagerLogic/TaskManagerComponent.RemoveSpawnedTask` _taskmanager (`self.ID_Task`))
      (`/Game/PrototypeLogic/Core/Managers/TaskManagerLogic/TaskManagerComponent.UnHideSpawnedTasks` _taskmanager)
      (`/Game/PrototypeLogic/Core/Managers/TaskManagerLogic/TaskManagerComponent.SetVisibleTaskControlButtons` _taskmanager false))
    (:`then_2`
      (`self.DestroySpawnedActors`))))

(fn `DestroySpawnedActors`
  (bind _spawnedactorsmap (`self.SpawnedActorsMap`))
  (if (> (`BlueprintMapLibrary.Map_Length` _spawnedactorsmap) 0)
    (bind _values (`BlueprintMapLibrary.Map_Values` _spawnedactorsmap))
    (for _array_element _values
      (`self.DestroyMe` _array_element))))

(fn `HideDescriptionTaskPopup`
  (`/Game/PrototypeLogic/Core/WidgetLogic/HUD/HUD_Information.RemoveTaskPopupBaseFromHUD` (`/Game/PrototypeLogic/Core/Player/BP_MainGameMode.InformationHUD` (`self.MainGameMode`))))

(fn `HideTask`
  (`SceneComponent.SetVisibility` (`self.TaskMesh`) false false)
  (`PrimitiveComponent.SetCollisionEnabled` (`self.TaskMesh`) "NoCollision")
  (`PrimitiveComponent.SetCollisionEnabled` (`self.TriggerTask`) "NoCollision"))

(fn `InitAdditionTasks`
  (bind _additiontasks (`self.AdditionTasks`))
  (if (> (`KismetArrayLibrary.Array_Length` _additiontasks) 0)
    (for _array_element _additiontasks
      (`/Game/PrototypeLogic/Core/Managers/TaskManagerLogic/BaseLogic/Task_Base.InitTask` _array_element))
    (`self.DebugLog` "Parent:Init Addition Tasks")))

(fn `InitMainTasks`
  (for _array_element (`self.MainTasks`)
    (`/Game/PrototypeLogic/Core/Managers/TaskManagerLogic/BaseLogic/Task_Base.InitTask` _array_element)))

(fn `InitTask`
  (bind _taskmanager (`self.TaskManager`))
  (`/Game/PrototypeLogic/Core/Managers/TaskManagerLogic/TaskManagerComponent.SetCurrentTask` _taskmanager (`self.ID_Task`))
  (`/Game/PrototypeLogic/Core/Managers/TaskManagerLogic/TaskManagerComponent.HideSpawnedTasks` _taskmanager))

(fn `Interact`
  (`parent.Interact`)
  (if (not (`self.bIsTaskActive`))
    (`self.InitTask`)))

(fn `Preview`
  (`self.DebugLog` "Parent:Preview"))

(fn `ReloadAdditionTasks`
  (bind _additiontasks (`self.AdditionTasks`))
  (if (> (`KismetArrayLibrary.Array_Length` _additiontasks) 0)
    (for _array_element _additiontasks
      (`/Game/PrototypeLogic/Core/Managers/TaskManagerLogic/BaseLogic/Task_Base.ReloadTask` _array_element))
    (`self.DebugLog` "Parent:Reload Addition Tasks")))

(fn `ReloadMainTasks`
  (for _array_element (`self.MainTasks`)
    (`/Game/PrototypeLogic/Core/Managers/TaskManagerLogic/BaseLogic/Task_Base.ReloadTask` _array_element)))

(fn `ReloadTask`
  (bind _spawnedactorsmap (`self.SpawnedActorsMap`))
  (`self.DebugLog` "Parent:Reload")
  (`|ExecutionSequence`
    (:`then_0`
      (`self.RemoveInteractionText`)
      (`self.ReloadMainTasks`)
      (`self.ReloadAdditionTasks`))
    (:`then_1`
      ;[1 1 1] Reload Spawned Actors
      (if (> (`BlueprintMapLibrary.Map_Length` _spawnedactorsmap) 0)
        (bind _values (`BlueprintMapLibrary.Map_Values` _spawnedactorsmap))
        (for _array_element _values
          (`self.ReloadMe` _array_element))))
    (:`then_2`
      (`self.StartTask`))
    (:`then_3`
      (`self.OnTaskReloaded`))))

(fn `RemoveInteractionText`
  (`/Game/PrototypeLogic/Core/WidgetLogic/HUD/HUD_Information.RemoveInterationInformation` (`/Game/PrototypeLogic/Core/Player/BP_MainGameMode.InformationHUD` (`self.MainGameMode`))))

(fn `ResetMainTaskValues`
  (`/Game/PrototypeLogic/Core/WidgetLogic/Popups/Task/DescriptionTask_Popup.ResetValues` (`/Game/PrototypeLogic/Core/Managers/TaskManagerLogic/TaskManagerComponent.DescriptionGeneralTaskPopup` (`/Game/PrototypeLogic/Core/Player/BP_MainGameMode.TaskManagerComponent` (`self.MainGameMode`)))))

(fn `RestoreTask`
  (`self.DebugLog` "Parent:RestoredTask"))

(fn `SaveTask`
  (`self.DebugLog` "Parent:SavedTask"))

(fn `ShowAdditionTasksPopup`
  (`/Game/PrototypeLogic/Core/Managers/PopupManagerLogic/PopupManagerComponent.AddToQueue` (`/Game/PrototypeLogic/Core/Player/BP_MainGameMode.PopupManagerComponent` (`self.MainGameMode`)) (`/Game/PrototypeLogic/Core/Managers/TaskManagerLogic/TaskManagerComponent.AdditionTasksPopup` (`/Game/PrototypeLogic/Core/Player/BP_MainGameMode.TaskManagerComponent` (`self.MainGameMode`)))))

(fn `ShowDescriptionTaskPopup`
  (`/Game/PrototypeLogic/Core/WidgetLogic/Popups/Task/DescriptionTask_Popup.SetDescriptionTaskName` (`/Game/PrototypeLogic/Core/Managers/TaskManagerLogic/TaskManagerComponent.DescriptionGeneralTaskPopup` (`self.TaskManager`)) (`self.TitleName`))
  (`/Game/PrototypeLogic/Core/WidgetLogic/Popups/Task/DescriptionTask_Popup.SetDescriptionTaskImage` (`/Game/PrototypeLogic/Core/Managers/TaskManagerLogic/TaskManagerComponent.DescriptionGeneralTaskPopup` (`self.TaskManager`)) (`self.TitleImage`))
  (`/Game/PrototypeLogic/Core/WidgetLogic/Popups/Task/DescriptionTask_Popup.SetDescriptionTaskPart` (`/Game/PrototypeLogic/Core/Managers/TaskManagerLogic/TaskManagerComponent.DescriptionGeneralTaskPopup` (`self.TaskManager`)) (`self.TitlePart`))
  (`/Game/PrototypeLogic/Core/WidgetLogic/HUD/HUD_Information.AddTaskPopupBaseToHUD` (`/Game/PrototypeLogic/Core/Player/BP_MainGameMode.InformationHUD` (`self.MainGameMode`)) (`/Game/PrototypeLogic/Core/Managers/TaskManagerLogic/TaskManagerComponent.DescriptionGeneralTaskPopup` (`self.TaskManager`))))

(fn `ShowFinishedTaskPopup`
  (bind _completedtaskpopup (`/Game/PrototypeLogic/Core/Managers/TaskManagerLogic/TaskManagerComponent.CompletedTaskPopup` (`self.TaskManager`)))
  (`/Game/PrototypeLogic/Core/WidgetLogic/Popups/Task/CompleteTask_Popup.ClearAdditionTasksInfo` _completedtaskpopup)
  (`/Game/PrototypeLogic/Core/WidgetLogic/Popups/Task/CompleteTask_Popup.SetMainTaskImage` _completedtaskpopup (`self.TitleImage`))
  (`/Game/PrototypeLogic/Core/WidgetLogic/Popups/Task/CompleteTask_Popup.SetMainTaskName` _completedtaskpopup (`self.TitleName`))
  (`/Game/PrototypeLogic/Core/WidgetLogic/Popups/Task/CompleteTask_Popup.SetMainTaskPart` _completedtaskpopup (`self.TitlePart`))
  (for _array_element (`self.AdditionTasks`)
    (`/Game/PrototypeLogic/Core/WidgetLogic/Popups/Task/CompleteTask_Popup.AddAdditionTaskInfo` _completedtaskpopup (`/Game/PrototypeLogic/Core/Managers/TaskManagerLogic/BaseLogic/Task_Base.TaskRaw` _array_element)))
  (`UserWidget.AddToViewport` _completedtaskpopup 0))

(fn `SpawnActor`
  (params (SpawnClass :type "/Game/PrototypeLogic/Core/Managers/BP_BaseActor Class Reference") (SpawnName :type String) (SpawnID :type Integer) (Transform :type "Transform Structure"))
  (returns (ReturnValue :type "/Game/PrototypeLogic/Core/Managers/BP_BaseActor Object Reference"))
  (bind _returnvalue (`|SpawnActorFromClass` SpawnClass Transform "Undefined" "OverrideRootScale" null null))
  (set `/Game/PrototypeLogic/Core/Managers/BP_BaseActor.ID_Actor` SpawnID _returnvalue)
  (`BlueprintMapLibrary.Map_Add` (`self.SpawnedActorsMap`) SpawnName _returnvalue)
  (return _returnvalue))

(fn `StartAdditionTaskModule`
  (params (TaskName :type Name))
  (bind (_value _returnvalue) (`BlueprintMapLibrary.Map_Find` (`self.AdditionTasksGroup`) TaskName))
  (if _returnvalue
    (`/Game/PrototypeLogic/Core/Managers/TaskManagerLogic/BaseLogic/Task_Base.StartTask` _value)
    (else
      ;[1 1 1] DebugMessage
      (bind _output_get (set `self.DebugText` "Didn't find "))
      (`self.ErrorLog` (`KismetStringLibrary.Concat_StrStr` (`KismetStringLibrary.Concat_StrStr` _output_get (`KismetStringLibrary.Conv_NameToString` TaskName)) " in AdditionTasksGroup")))))

(fn `StartMainTaskModule`
  (params (TaskName :type Name))
  (bind (_value _returnvalue) (`BlueprintMapLibrary.Map_Find` (`self.MainTasksGroup`) TaskName))
  (if _returnvalue
    (`/Game/PrototypeLogic/Core/Managers/TaskManagerLogic/BaseLogic/Task_Base.StartTask` _value)
    (else
      ;[1 1 1] DebugMessage
      (bind _output_get (set `self.DebugText` "Didn't find "))
      (`self.ErrorLog` (`KismetStringLibrary.Concat_StrStr` (`KismetStringLibrary.Concat_StrStr` _output_get (`KismetStringLibrary.Conv_NameToString` TaskName)) " in MainTasksGroup")))))

(fn `StartTask`
  (locals (TaskHUDLocal :type "/Game/PrototypeLogic/Core/WidgetLogic/BaseLogic/HUD_Base Object Reference"))
  (bind _maingamemode (`self.MainGameMode`))
  (`self.DebugLog` "Parent:Start")
  (set `self.bIsTaskActive` true)
  (`/Game/PrototypeLogic/Core/Managers/TaskManagerLogic/BaseLogic/Task_Base.StartTask` (`|GetArrayItem` (`self.MainTasks`)))
  (`/Game/PrototypeLogic/Core/Managers/TaskManagerLogic/TaskManagerComponent.SetVisibleTaskControlButtons` (`self.TaskManager`) true)
  (`/Game/PrototypeLogic/Core/WidgetLogic/HUD/HUD_Information.AddTaskPopupBaseToHUD` (`/Game/PrototypeLogic/Core/Player/BP_MainGameMode.InformationHUD` _maingamemode) (`/Game/PrototypeLogic/Core/Managers/TaskManagerLogic/TaskManagerComponent.MainTaskPopup` (`/Game/PrototypeLogic/Core/Player/BP_MainGameMode.TaskManagerComponent` _maingamemode)))
  (`self.DebugLog` "STARTED"))

(fn `UnHideTask`
  (`SceneComponent.SetVisibility` (`self.TaskMesh`) true false)
  (`PrimitiveComponent.SetCollisionEnabled` (`self.TaskMesh`) "QueryAndPhysics")
  (`PrimitiveComponent.SetCollisionEnabled` (`self.TriggerTask`) "QueryAndPhysics"))

(fn `UserConstructionScript`
  (bind _maingamemode (`self.MainGameMode`))
  (`parent.UserConstructionScript`)
  (set `self.UIManager` (`/Game/PrototypeLogic/Core/Player/BP_MainGameMode.UIManagerComponent` _maingamemode))
  (set `self.TaskManager` (`/Game/PrototypeLogic/Core/Player/BP_MainGameMode.TaskManagerComponent` _maingamemode))
  (`|ExecutionSequence`
    (:`then_0`
      (bind _output_get (set `self.AdditionTasks` (`self.K2_GetComponentsByClass` "/Game/PrototypeLogic/Core/Managers/TaskManagerLogic/BaseLogic/AdditionTask_Base.AdditionTask_Base_C")))
      (for _array_element _output_get
        (`BlueprintMapLibrary.Map_Add` (`self.AdditionTasksGroup`) (`/Game/PrototypeLogic/Core/Managers/TaskManagerLogic/BaseLogic/Task_Base.TaskName` _array_element) _array_element)))
    (:`then_1`
      (bind _output_get_2 (set `self.MainTasks` (`self.K2_GetComponentsByClass` "/Game/PrototypeLogic/Core/Managers/TaskManagerLogic/BaseLogic/MainTask_Base.MainTask_Base_C")))
      (for _array_element_2 _output_get_2
        (`BlueprintMapLibrary.Map_Add` (`self.MainTasksGroup`) (`/Game/PrototypeLogic/Core/Managers/TaskManagerLogic/BaseLogic/Task_Base.TaskName` _array_element_2) _array_element_2)))))