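; Base actor class that links its instances to the tick and debug manager components on BP_MainGameMode.
; The construction script caches the game mode, registers CanTick actors with the tick manager, stores the start transform and marks the actor active.
; DestroyMe and Destroyed unregister tickable actors, while HideMe and UnHideMe only toggle the active flag.
; Log helpers forward messages to the debug manager, and ReloadMe is an empty stub.
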(event `self.ReceiveBeginPlay`)

(event `self.ReceiveDestroyed`
  (if (`self.bCanTick`)
    (`/Game/PrototypeLogic/Core/Managers/TickManagerLogic/TickManagerComponent.RemoveTickableObject` (`/Game/PrototypeLogic/Core/Player/BP_MainGameMode.TickManagerComponent` (`self.MainGameMode`)) self)))

(fn `DebugLog`
  (params (Message :type String))
  (`/Game/PrototypeLogic/Core/Managers/DebugManagerLogic/DebugManagerComponent.DebugLog` (`/Game/PrototypeLogic/Core/Player/BP_MainGameMode.DebugManagerComponent` (`self.MainGameMode`)) self Message))

(fn `DestroyMe`
  (`|ExecutionSequence`
    (:`then_0`
      (if (`self.bCanTick`)
        (`/Game/PrototypeLogic/Core/Managers/TickManagerLogic/TickManagerComponent.RemoveTickableObject` (`/Game/PrototypeLogic/Core/Player/BP_MainGameMode.TickManagerComponent` (`self.MainGameMode`)) self)
        (`self.DebugLog` "Removed Tickable")))
    (:`then_1`
      (`self.DebugLog` "Destroyed")
      (`self.K2_DestroyActor` self))))

(fn `ErrorLog`
  (params (Message :type String))
  (`/Game/PrototypeLogic/Core/Managers/DebugManagerLogic/DebugManagerComponent.ErrorLog` (`/Game/PrototypeLogic/Core/Player/BP_MainGameMode.DebugManagerComponent` (`self.MainGameMode`)) self Message))

(fn `HideMe`
  (set `self.bIsActorActive` false))

(fn `ReloadMe`)

(fn `SuccessLog`
  (params (Message :type String))
  (`/Game/PrototypeLogic/Core/Managers/DebugManagerLogic/DebugManagerComponent.SuccessLog` (`/Game/PrototypeLogic/Core/Player/BP_MainGameMode.DebugManagerComponent` (`self.MainGameMode`)) self Message))

(fn `UnHideMe`
  (set `self.bIsActorActive` true))

(fn `UserConstructionScript`
  (`|ExecutionSequence`
    (:`then_0`
      (bind _asbp_main_game_mode (cast `/Game/PrototypeLogic/Core/Player/BP_MainGameMode` (`GameplayStatics.GetGameMode`)))
      (set `self.MainGameMode` _asbp_main_game_mode))
    (:`then_1`
      (if (`self.bCanTick`)
        (`/Game/PrototypeLogic/Core/Managers/TickManagerLogic/TickManagerComponent.AddTickableObject` (`/Game/PrototypeLogic/Core/Player/BP_MainGameMode.TickManagerComponent` (`self.MainGameMode`)) self)))
    (:`then_2`
      (set `self.StartActorTransform` (`self.GetTransform`)))
    (:`then_3`
      (set `self.bIsActorActive` true))))

(fn `WarningLog`
  (params (Message :type String))
  (`/Game/PrototypeLogic/Core/Managers/DebugManagerLogic/DebugManagerComponent.WarningLog` (`/Game/PrototypeLogic/Core/Player/BP_MainGameMode.DebugManagerComponent` (`self.MainGameMode`)) self Message))